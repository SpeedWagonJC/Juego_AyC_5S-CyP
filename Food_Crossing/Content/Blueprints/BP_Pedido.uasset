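; BP_Pedido is an order ("pedido") actor that the player completes by bringing a matching inventory.
; Its Box overlap events track whether an actor tagged Player is nearby and cache the Player reference.
; On F_Interact, it requires the player's inventory array to be identical to Pedido, then destroys itself.
; Spanish debug prints report success, a wrong inventory or being too far away, and failure changes nothing.
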(event `self.ReceiveBeginPlay`)

(event `InputAction|F_Interact`
  (params (Key :type "Key Structure"))
  (:`Pressed`
    (if (`self.Is_Player_Near`)
      (bind _p_pedido (`/Game/Player/Player.Get_Inventory` (`self.As Player`)))
      (if (`KismetArrayLibrary.Array_Identical` _p_pedido (`self.Pedido`))
        (`KismetSystemLibrary.PrintString` "Pedido completado!!!!")
        (`self.K2_DestroyActor`)
        (else
          (`KismetSystemLibrary.PrintString` "ESTA MAL!!!!!")))
      (else
        (`KismetSystemLibrary.PrintString` "Acercate vieja")))))

(event `self.Box.OnComponentBeginOverlap`
  (params (OverlappedComponent :type "PrimitiveComponent Object Reference") (OtherActor :type "Actor Object Reference") (OtherComp :type "PrimitiveComponent Object Reference") (OtherBodyIndex :type Integer) (bFromSweep :type Boolean) (SweepResult :type "HitResult Structure (by ref)"))
  ;[0.15 0.04547 0.04021 0.5] Is player near
  (if (`self.ActorHasTag` OtherActor "Player")
    (bind _asplayer (cast `/Game/Player/Player` OtherActor))
    (set `self.Is_Player_Near` true)
    (set `self.As Player` _asplayer)))

(event `self.Box.OnComponentEndOverlap`
  (params (OverlappedComponent :type "PrimitiveComponent Object Reference") (OtherActor :type "Actor Object Reference") (OtherComp :type "PrimitiveComponent Object Reference") (OtherBodyIndex :type Integer))
  ;[0.15 0.04547 0.04021 0.5] Is player near
  (if (`self.ActorHasTag` OtherActor "Player")
    (cast `/Game/Player/Player` OtherActor)
    (set `self.Is_Player_Near` false)))

(fn `UserConstructionScript`)