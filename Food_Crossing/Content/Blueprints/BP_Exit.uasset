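; BP_Exit is an exit trigger that loads the City level when the player stands near it and presses G.
; A box component's overlap events set and clear IsPlayerNear for actors tagged Player that also cast to the Player class.
; Pressing G opens the level by object reference if the flag is set, and otherwise prints a Spanish message telling the player to come closer.
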(event `Key|G`
  (params (Key :type "Key Structure"))
  ;[0 0.03822 0.6927 0.5] Open Level
  (:`Pressed`
    (if (`self.IsPlayerNear`)
      (`GameplayStatics.OpenLevelBySoftObjectPtr` "/Game/City.City")
      (else
        (`KismetSystemLibrary.PrintString` "Acercate viejo")))))

(event `self.Box.OnComponentBeginOverlap`
  (params (OverlappedComponent :type "PrimitiveComponent Object Reference") (OtherActor :type "Actor Object Reference") (OtherComp :type "PrimitiveComponent Object Reference") (OtherBodyIndex :type Integer) (bFromSweep :type Boolean) (SweepResult :type "HitResult Structure (by ref)"))
  ;[0 0.01565 0.151 0.5] Is Player Near
  (if (`self.ActorHasTag` OtherActor "Player")
    (cast `/Game/Player/Player` OtherActor)
    (set `self.IsPlayerNear` true)))

(event `self.Box.OnComponentEndOverlap`
  (params (OverlappedComponent :type "PrimitiveComponent Object Reference") (OtherActor :type "Actor Object Reference") (OtherComp :type "PrimitiveComponent Object Reference") (OtherBodyIndex :type Integer))
  ;[0 0.01565 0.151 0.5] Is Player Near
  (if (`self.ActorHasTag` OtherActor "Player")
    (cast `/Game/Player/Player` OtherActor)
    (set `self.IsPlayerNear` false)))

(fn `UserConstructionScript`)